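; Modular platform cell that builds a configurable room tile, with optional walls, ceiling, light and a trap or reward.
; The construction script scales the floor by GridSize and spawns cube meshes for enabled walls and ceiling; light placement and child-actor trap/reward selection run only with a ceiling.
; At runtime, the player's GotHit dispatcher triggers a timeline-driven light color flash.
; Wall_Side temporarily swaps every wall's material for three seconds.
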(event `Wall_Side`
  (for _array_element (`self.Walls`)
    (`PrimitiveComponent.SetMaterial` _array_element 0 "/Game/materials/metal1.metal1"))
  (`KismetSystemLibrary.Delay` 3.0)
  (for _array_element_2 (`self.Walls`)
    (`PrimitiveComponent.SetMaterial` _array_element_2 0 "/Game/materials/metal.metal")))

(event `self.ReceiveBeginPlay`
  (bind _asbp_first_person_character (cast `/Game/blueprints/BP_FirstPersonCharacter` (`GameplayStatics.GetPlayerCharacter` 0)))
  (bind _output_get (set `self.As BP First Person Character` _asbp_first_person_character))
  (add `/Game/blueprints/BP_FirstPersonCharacter.DP_GotHit` _output_get (delegate `Light_Update`)))

(event `Light_Update`
  (params (HP :type "Float (double-precision)"))
  (bind (_default_light_color_b _default_light_color_g _default_light_color_r) (break `Color` (`self.Default_Light_Color`)))
  (if (> (`self.Light_Intensity`) 0.0)
    (if (not (`self.Timeline_Active`))
      (bind (_direction _default_light_multiplyer _red) (`Timeline|Timeline` :!via `PlayFromStart`)
        (:`Update`
          (set `self.Timeline_Active` true)
          (`LightComponent.SetLightColor` (`self.PointLight`) (make `LinearColor` (`KismetMathLibrary.Abs` (- _red (/ _default_light_color_r 255))) (* (/ _default_light_color_g 255) _default_light_multiplyer) (* (/ _default_light_color_b 255) _default_light_multiplyer)) true))
        (:`Finished`
          (set `self.Timeline_Active` false))))))

(fn `UserConstructionScript`
  (bind _gridsize (`self.GridSize`))
  (bind _gridsize_2 (`self.GridSize`))
  (bind _gridsize_3 (`self.GridSize`))
  (bind _gridsize_4 (`self.GridSize`))
  (bind _gridsize_5 (`self.GridSize`))
  (bind _gridsize_6 (`self.GridSize`))
  (bind _gridsize_7 (`self.GridSize`))
  (bind _gridsize_8 (`self.GridSize`))
  (bind _gridsize_9 (`self.GridSize`))
  (bind _gridsize_10 (`self.GridSize`))
  (bind _returnvalue (* (`self.GridSize`) -50.0))
  (bind (_relativelocation_x _relativelocation_y _relativelocation_z) (`KismetMathLibrary.BreakVector` (`SceneComponent.RelativeLocation` (`self.Plane`))))
  (bind (_relativelocation_x_2 _relativelocation_y_2 _relativelocation_z_2) (`KismetMathLibrary.BreakVector` (`SceneComponent.RelativeLocation` (`self.Plane`))))
  (`SceneComponent.SetRelativeScale3D` (`self.Plane`) (`KismetMathLibrary.MakeVector` _gridsize _gridsize 1.0))
  (`|ExecutionSequence`
    (:`then_0`
      (if (`self.South_Wall`)
        (bind _returnvalue_2 (`AddComponent|NODE_AddStaticMeshComponent-2` :`RelativeTransform` (`KismetMathLibrary.MakeTransform` (+ (`SceneComponent.RelativeLocation` (`self.Plane`)) (`KismetMathLibrary.MakeVector` (* _gridsize_3 -50.0) (* _gridsize_3 -50.0))) (struct) (`KismetMathLibrary.MakeVector` (* _gridsize_6 0.01) _gridsize_6 (`self.wall_height`)))))
        (`StaticMeshComponent.SetStaticMesh` _returnvalue_2 "/Game/LevelPrototyping/Meshes/SM_Cube.SM_Cube")
        (`PrimitiveComponent.SetMaterial` _returnvalue_2 0 "/Game/materials/metal.metal")
        (`KismetArrayLibrary.Array_Add` (`self.Walls`) _returnvalue_2)))
    (:`then_1`
      (if (`self.West_Wall`)
        (bind _returnvalue_3 (`AddComponent|NODE_AddStaticMeshComponent-3` :`RelativeTransform` (`KismetMathLibrary.MakeTransform` (+ (`SceneComponent.RelativeLocation` (`self.Plane`)) (`KismetMathLibrary.MakeVector` (* _gridsize_4 -50.0) (* _gridsize_4 -50.0))) (struct) (`KismetMathLibrary.MakeVector` _gridsize_7 (* _gridsize_7 0.01) (`self.wall_height`)))))
        (`StaticMeshComponent.SetStaticMesh` _returnvalue_3 "/Game/LevelPrototyping/Meshes/SM_Cube.SM_Cube")
        (`PrimitiveComponent.SetMaterial` _returnvalue_3 0 "/Game/materials/metal.metal")
        (`KismetArrayLibrary.Array_Add` (`self.Walls`) _returnvalue_3)))
    (:`then_2`
      (if (`self.North_Wall`)
        (bind _returnvalue_4 (`AddComponent|NODE_AddStaticMeshComponent-4` :`RelativeTransform` (`KismetMathLibrary.MakeTransform` (+ (`SceneComponent.RelativeLocation` (`self.Plane`)) (`KismetMathLibrary.MakeVector` (+ (* _gridsize_8 -1.0) (* _gridsize_8 50.0)) (* _gridsize_8 -50.0))) (struct) (`KismetMathLibrary.MakeVector` (* _gridsize_9 0.01) _gridsize_9 (`self.wall_height`)))))
        (`StaticMeshComponent.SetStaticMesh` _returnvalue_4 "/Game/LevelPrototyping/Meshes/SM_Cube.SM_Cube")
        (`PrimitiveComponent.SetMaterial` _returnvalue_4 0 "/Game/materials/metal.metal")
        (`KismetArrayLibrary.Array_Add` (`self.Walls`) _returnvalue_4)))
    (:`then_3`
      (if (`self.East_Wall`)
        (bind _returnvalue_5 (`AddComponent|NODE_AddStaticMeshComponent-5` :`RelativeTransform` (`KismetMathLibrary.MakeTransform` (+ (`SceneComponent.RelativeLocation` (`self.Plane`)) (`KismetMathLibrary.MakeVector` (* _gridsize_2 -50.0) (+ (* _gridsize_2 -1.0) (* _gridsize_2 50.0)))) (struct) (`KismetMathLibrary.MakeVector` _gridsize_5 (* _gridsize_5 0.01) (`self.wall_height`)))))
        (`StaticMeshComponent.SetStaticMesh` _returnvalue_5 "/Game/LevelPrototyping/Meshes/SM_Cube.SM_Cube")
        (`PrimitiveComponent.SetMaterial` _returnvalue_5 0 "/Game/materials/metal.metal")
        (`KismetArrayLibrary.Array_Add` (`self.Walls`) _returnvalue_5)))
    (:`then_4`
      (if (`self.HasCeiling`)
        (bind _returnvalue_6 (`AddComponent|NODE_AddStaticMeshComponent-6` :`RelativeTransform` (`KismetMathLibrary.MakeTransform` (`KismetMathLibrary.MakeVector` (+ _relativelocation_x_2 _returnvalue) (+ _relativelocation_y_2 _returnvalue) (+ _relativelocation_z_2 (* (`self.wall_height`) 100.0))) (struct) (`KismetMathLibrary.MakeVector` _gridsize_10 _gridsize_10 0.1))))
        (`StaticMeshComponent.SetStaticMesh` _returnvalue_6 "/Game/LevelPrototyping/Meshes/SM_Cube.SM_Cube")
        (bind _output_get (set `self.Light` (`self.PointLight`)))
        (`SceneComponent.K2_SetRelativeLocation` _output_get (`KismetMathLibrary.MakeVector` _relativelocation_x _relativelocation_y (+ _relativelocation_z (* (`self.wall_height`) 100.0) -20.0)) false false)
        (if (`self.HasCeiling`)
          (`LightComponent.SetIntensity` _output_get (`self.Light_Intensity`))
          (else
            (`LightComponent.SetIntensity` _output_get 0.0)))
        (if (`self.Can_Have_Objects`)
          (if (`self.Trap_or_reward`)
            (`ChildActorComponent.SetChildActorClass` (`self.Trap`) (select `int` (`self.trap_selection_index`) :`0` "/Game/blueprints/BP_SpikeTrap.BP_SpikeTrap_C" :`1` "/Game/blueprints/BP_Poison_Trap.BP_Poison_Trap_C" :`2` "/Game/blueprints/BP_Pendulum_Trap.BP_Pendulum_Trap_C" :`3` null :!type "Actor Class Reference"))
            (else
              (`ChildActorComponent.SetChildActorClass` (`self.reward`) (select `int` (`self.reward_selection_index`) :`0` "/Game/blueprints/BP_GoldPile.BP_GoldPile_C" :`1` "/Game/blueprints/Health_Pack.Health_Pack_C" :!type "Actor Class Reference")))))))))