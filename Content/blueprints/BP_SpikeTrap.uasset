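; BP_SpikeTrap is a floor trap that raises spikes when the first-person player enters its trigger and damages them on contact with the spike hitbox.
; A timeline drives the spike mesh's vertical offset.
; The construction script scales the parts from the parent BP_Platfrom_Cell's GridSize.
; A BP_Trap_Disabler with target index 0 can switch off the raising, but hitbox damage does not check the enabled flag.
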(event `self.ReceiveBeginPlay`
  (bind _asbp_first_person_character (cast `/Game/blueprints/BP_FirstPersonCharacter` (`GameplayStatics.GetPlayerCharacter` 0)))
  (set `self.As BP First Person Character` _asbp_first_person_character)
  (bind _outactors (`GameplayStatics.GetAllActorsOfClass` "/Game/blueprints/BP_Trap_Disabler.BP_Trap_Disabler_C"))
  (for _array_element _outactors
    (if (== (`/Game/blueprints/BP_Trap_Disabler.Target_trap_index` _array_element) 0)
      (set `self.Disabler_Ref` _array_element)))
  (add `/Game/blueprints/BP_Trap_Disabler.Traps_Disabled` (`self.Disabler_Ref`) (delegate `disabled`)))

(event `disabled`
  (params (Trap_Target_Index :type Integer))
  (if (== Trap_Target_Index 0)
    (set `self.Is_Enabled` false)))

(event `self.trap_trigger.OnComponentBeginOverlap`
  (params (OverlappedComponent :type "PrimitiveComponent Object Reference") (OtherActor :type "Actor Object Reference") (OtherComp :type "PrimitiveComponent Object Reference") (OtherBodyIndex :type Integer) (bFromSweep :type Boolean) (SweepResult :type "HitResult Structure (by ref)"))
  (bind (_returnvalue_x _returnvalue_y _returnvalue_z) (`KismetMathLibrary.BreakVector` (* (`SceneComponent.GetUpVector` (`self.OPM0041`)) (0.0 0.0 0.0))))
  (if (== OtherActor (`self.As BP First Person Character`))
    (if (`self.Is_Enabled`)
      (bind (_direction _newtrack_0) (`Timeline|Timeline` :!via `PlayFromStart`)
        (:`Update`
          (`SceneComponent.K2_SetRelativeLocation` (`self.OPM0041`) (`KismetMathLibrary.MakeVector` _returnvalue_x _returnvalue_y (+ (* _newtrack_0 10.0) _returnvalue_z)) false false))))))

(event `self.spike_hitbox.OnComponentBeginOverlap`
  (params (OverlappedComponent :type "PrimitiveComponent Object Reference") (OtherActor :type "Actor Object Reference") (OtherComp :type "PrimitiveComponent Object Reference") (OtherBodyIndex :type Integer) (bFromSweep :type Boolean) (SweepResult :type "HitResult Structure (by ref)"))
  (bind _as_bp_first_person_character (`self.As BP First Person Character`))
  (if (== OtherActor _as_bp_first_person_character)
    (`/Game/blueprints/BP_FirstPersonCharacter.Damage_Function` _as_bp_first_person_character (`self.Spike_Damage`))))

(fn `Get_Interact_State`
  (returns (InteractState :type Boolean))
  (return false))

(fn `UserConstructionScript`
  (bind _opm0041 (`self.OPM0041`))
  (bind _asbp_platfrom_cell (cast `/Game/blueprints/BP_Platfrom_Cell` (`self.GetParentActor`)))
  (bind _gridsize (`/Game/blueprints/BP_Platfrom_Cell.GridSize` _asbp_platfrom_cell))
  (bind _returnvalue (* _gridsize 1.0))
  (`SceneComponent.SetRelativeScale3D` (`self.Cube`) (`KismetMathLibrary.MakeVector` _returnvalue _returnvalue 0.1))
  (bind _returnvalue_2 (* _gridsize 1.5))
  (`SceneComponent.SetRelativeScale3D` (`self.trap_trigger`) (`KismetMathLibrary.MakeVector` _returnvalue_2 _returnvalue_2 1.0))
  (`SceneComponent.SetRelativeScale3D` _opm0041 (`KismetMathLibrary.MakeVector` _returnvalue _returnvalue 5.0))
  (`SceneComponent.K2_SetRelativeLocation` _opm0041 (0.0 0.0 -100.0) false false))