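; Swinging sword pendulum trap, built as a child actor of BP_Platfrom_Cell, that damages the first-person player.
; Construction sizes and positions the sword and trigger box from the parent cell's grid size, wall height and trap rotation.
; Player overlap with the trigger plays one timeline-driven swing at a time, while sword box overlap applies damage.
; A BP_Trap_Disabler with trap index 1 switches off further triggering through an event.
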(event `self.ReceiveBeginPlay`
  (bind _asbp_first_person_character (cast `/Game/blueprints/BP_FirstPersonCharacter` (`GameplayStatics.GetPlayerCharacter` 0)))
  (set `self.As BP First Person Character` _asbp_first_person_character)
  (add `PrimitiveComponent.OnComponentBeginOverlap` (`self.Trigger_box`) (delegate `OnComponentBeginOverlap_Event`))
  (add `PrimitiveComponent.OnComponentBeginOverlap` (`self.Sword_box`) (delegate `Sword_hit`))
  (bind _outactors (`GameplayStatics.GetAllActorsOfClass` "/Game/blueprints/BP_Trap_Disabler.BP_Trap_Disabler_C"))
  (for _array_element _outactors
    (if (== (`/Game/blueprints/BP_Trap_Disabler.Target_trap_index` _array_element) 1)
      (set `self.Disabler_ref` _array_element)))
  (add `/Game/blueprints/BP_Trap_Disabler.Traps_Disabled` (`self.Disabler_ref`) (delegate `Disabled`)))

(event `Sword_hit`
  (params (OverlappedComponent :type "PrimitiveComponent Object Reference") (OtherActor :type "Actor Object Reference") (OtherComp :type "PrimitiveComponent Object Reference") (OtherBodyIndex :type Integer) (bFromSweep :type Boolean) (SweepResult :type "HitResult Structure (by ref)"))
  (bind _as_bp_first_person_character (`self.As BP First Person Character`))
  (if (== OtherActor _as_bp_first_person_character)
    (`/Game/blueprints/BP_FirstPersonCharacter.Damage_Function` _as_bp_first_person_character (`self.Sword_damage`))))

(event `Disabled`
  (params (Trap_Target_Index :type Integer))
  (if (== Trap_Target_Index 1)
    (set `self.Is_Enabled` false)))

(event `OnComponentBeginOverlap_Event`
  (params (OverlappedComponent :type "PrimitiveComponent Object Reference") (OtherActor :type "Actor Object Reference") (OtherComp :type "PrimitiveComponent Object Reference") (OtherBodyIndex :type Integer) (bFromSweep :type Boolean) (SweepResult :type "HitResult Structure (by ref)"))
  (bind (_trap_rotation_roll _trap_rotation_pitch _trap_rotation_yaw) (`KismetMathLibrary.BreakRotator` (`/Game/blueprints/BP_Platfrom_Cell.Trap_Rotation` (`self.Cell_Ref`))))
  (if (`self.Is_Enabled`)
    (if (`self.Trap_active`)
      _
      (elif (== OtherActor (`self.As BP First Person Character`))
        (bind (_direction _newtrack_0) (`Timeline|Swing` :!via `PlayFromStart`)
          (:`Update`
            (set `self.Trap_active` true)
            (`SceneComponent.K2_SetRelativeRotation` (`self.sworb`) (`KismetMathLibrary.MakeRotator` (+ (* _newtrack_0 45.0) 0.0) 180.0 _trap_rotation_yaw) false false))
          (:`Finished`
            (set `self.Trap_active` false)))))))

(fn `Get_Interact_State`
  (returns (InteractState :type Boolean))
  (return false))

(fn `UserConstructionScript`
  (bind _sworb (`self.sworb`))
  (bind _trigger_box (`self.Trigger_box`))
  (bind _cell_ref (`self.Cell_Ref`))
  (bind _wall_height (`/Game/blueprints/BP_Platfrom_Cell.wall_height` _cell_ref))
  (bind (_trap_rotation_roll _trap_rotation_pitch _trap_rotation_yaw) (`KismetMathLibrary.BreakRotator` (`/Game/blueprints/BP_Platfrom_Cell.Trap_Rotation` (`self.Cell_Ref`))))
  (bind _returnvalue (* (`/Game/blueprints/BP_Platfrom_Cell.GridSize` _cell_ref) 1.5))
  (bind _asbp_platfrom_cell (cast `/Game/blueprints/BP_Platfrom_Cell` (`self.GetParentActor`)))
  (bind _output_get (set `self.Cell_Ref` _asbp_platfrom_cell))
  (`|ExecutionSequence`
    (:`then_0`
      (bind _wall_height_2 (`/Game/blueprints/BP_Platfrom_Cell.wall_height` _output_get))
      (`SceneComponent.K2_SetRelativeLocation` _sworb (`KismetMathLibrary.MakeVector` 0.0 0.0 (+ (* _wall_height_2 90.0) -20.0)) false false)
      (`SceneComponent.SetRelativeScale3D` _sworb (`KismetMathLibrary.Conv_DoubleToVector` (* _wall_height_2 0.04)))
      (`SceneComponent.K2_SetRelativeRotation` _sworb (`KismetMathLibrary.MakeRotator` 45.0 _trap_rotation_pitch _trap_rotation_yaw) false false))
    (:`then_1`
      (`SceneComponent.SetRelativeScale3D` _trigger_box (`KismetMathLibrary.MakeVector` _returnvalue _returnvalue _wall_height))
      (`SceneComponent.K2_SetRelativeLocation` _trigger_box (`KismetMathLibrary.MakeVector` 0.0 0.0 (* _wall_height 50.0)) false false))))